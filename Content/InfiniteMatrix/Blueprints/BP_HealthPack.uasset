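; BP_HealthPack is a short-lived pickup actor that heals the player and destroys itself five seconds after spawning.
; When BP_Player overlaps its Box, it shows a HealthNotification widget briefly, then removes the widget and destroys itself.
; Health is clamped to 0–100 before the fixed bonus is added, so the result can exceed 100.
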(event OnComponentBeginOverlap(Box)
  (params (OverlappedComponent :type Primitive%20Component%20Object%20Reference) (OtherActor :type Actor%20Object%20Reference) (OtherComp :type Primitive%20Component%20Object%20Reference) (OtherBodyIndex :type Integer) (bFromSweep :type Boolean) (SweepResult :type Hit%20Result%20Structure%20%28by%20ref%29))
  (bind _asbp_player (Utilities|Casting|CastToBP_Player OtherActor))
  (CallFunction|ShowHealthMessage)
  (Variables|/Game/InfiniteMatrix/Blueprints/BP_Player.BP_Player_C|SetHealth _asbp_player (+ (Math|Float|Clamp(Float) (Variables|/Game/InfiniteMatrix/Blueprints/BP_Player.BP_Player_C|GetHealth _asbp_player) 0.0 1e+02) 1e+01)))

(event Custom|ShowHealthMessage
  (bind _returnvalue (UserInterface|CreateWidget "/Game/InfiniteMatrix/UI/HealthNotification.HealthNotification_C"))
  (UserInterface|Viewport|AddtoViewport _returnvalue 0)
  (Utilities|FlowControl|Delay 0.5)
  (Widget|RemovefromParent _returnvalue)
  (Actor|DestroyActor))

(event EventBeginPlay
  (Utilities|FlowControl|Delay 5.0)
  (Actor|DestroyActor))

(event Collision|EventActorBeginOverlap
  (params (OtherActor :type Actor%20Object%20Reference)))

(event EventTick
  (params (DeltaSeconds :type Float%20%28single-precision%29)))

(fn ConstructionScript)